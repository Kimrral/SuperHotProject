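; VR player character that picks up, holds and throws a pistol, shotgun or Uzi, and animates both hands from XR input.
; The attach input box-traces for a weapon, resets its ammo, snaps it to a right-hand socket and hides the hand meshes.
; With a weapon equipped, the same input detaches it and launches it along the camera's forward vector.
; BeginPlay pre-spawns all three weapons below the origin; helper events handle bullet spawning and fire cooldown.
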(event Input|EnhancedActionEvents|EnhancedInputActionIA_Hand_Grasp_Left
  (params (ActionValue :type Float%20%28double-precision%29) (ElapsedSeconds :type Float%20%28double-precision%29) (TriggeredSeconds :type Float%20%28double-precision%29) (InputAction :type Input%20Action%20Object%20Reference :default "/Game/VRTemplate/Input/Actions/Hands/IA_Hand_Grasp_Left.IA_Hand_Grasp_Left"))
  (bind _lefthandmesh (Variables|Default|GetLeftHandMesh))
  (bind _returnvalue (Components|SkeletalMesh|GetAnimInstance _lefthandmesh))
  (:Triggered
    (bind _asabp_mannequins_xr (Utilities|Casting|CastToABP_MannequinsXR _returnvalue))
    (Variables|/Game/Characters/MannequinsXR/Meshes/ABP_MannequinsXR.ABP_MannequinsXR_C|SetPoseAlphaGrasp _asabp_mannequins_xr ActionValue))
  (:Canceled
    (bind _asabp_mannequins_xr_2 (Utilities|Casting|CastToABP_MannequinsXR _returnvalue :!label _label))
    (Variables|/Game/Characters/MannequinsXR/Meshes/ABP_MannequinsXR.ABP_MannequinsXR_C|SetPoseAlphaGrasp _asabp_mannequins_xr_2 0.0))
  (:Completed
    (goto _label)))

(event Input|EnhancedActionEvents|EnhancedInputActionIA_Attach
  (params (ActionValue :type Boolean) (ElapsedSeconds :type Float%20%28double-precision%29) (TriggeredSeconds :type Float%20%28double-precision%29) (InputAction :type Input%20Action%20Object%20Reference :default "/Game/FirstPerson/Input/Actions/IA_Attach.IA_Attach"))
  (bind (_returnvalue _returnvalue2) (|LineTraceLoc))
  (:Started
    (if (Variables|Default|GetisWeaponEquipped)
      (if (Variables|Default|GetisUsingShotgun)
        (Utilities|IsValid (Variables|Default|GetShotgunRef)
          (:Is%20Valid
            (Default|Throw (Variables|Default|GetShotgunRef))
            (Transformation|DetachFromActor (Variables|Default|GetShotgunRef) "KeepWorld" "KeepWorld" "KeepWorld")
            (Physics|AddImpulseatLocation (Variables|/Script/SuperHotProject.BaseWeapon|GetBoxComp (Variables|Default|GetShotgunRef)) "500.000000,0.000000,0.000000" (- (Transformation|GetWorldLocation (Variables|/Script/SuperHotProject.BaseWeapon|GetBoxComp (Variables|Default|GetShotgunRef))) "0.000000,10.000000,0.000000") "None")
            (Physics|AddImpulse (Variables|/Script/SuperHotProject.BaseWeapon|GetBoxComp (Variables|Default|GetShotgunRef)) (* (Math|Vector|GetForwardVector (Transformation|GetWorldRotation (Variables|Default|GetVRCamera))) (Variables|Default|GetThrowVelocity)) "None" true)
            (Variables|Default|SetShotgunRef 0)
            (Variables|Default|SetisWeaponEquipped false)
            (Variables|Default|SetisUsingShotgun false)
            (Variables|Default|SetisUsingUzi false)))
        (elif (Variables|Default|GetisUsingUzi)
          (Utilities|IsValid (Variables|Default|GetUziRef)
            (:Is%20Valid
              (Default|Throw (Variables|Default|GetUziRef))
              (Transformation|DetachFromActor (Variables|Default|GetUziRef) "KeepWorld" "KeepWorld" "KeepWorld")
              (Physics|AddImpulseatLocation (Variables|/Script/SuperHotProject.BaseWeapon|GetBoxComp (Variables|Default|GetUziRef)) "500.000000,0.000000,0.000000" (- (Transformation|GetWorldLocation (Variables|/Script/SuperHotProject.BaseWeapon|GetBoxComp (Variables|Default|GetUziRef))) "0.000000,10.000000,0.000000") "None")
              (Physics|AddImpulse (Variables|/Script/SuperHotProject.BaseWeapon|GetBoxComp (Variables|Default|GetUziRef)) (* (Math|Vector|GetForwardVector (Transformation|GetWorldRotation (Variables|Default|GetVRCamera))) (Variables|Default|GetThrowVelocity)) "None" true)
              (Variables|Default|SetUziRef 0)
              (Variables|Default|SetisWeaponEquipped false)
              (Variables|Default|SetisUsingShotgun false)
              (Variables|Default|SetisUsingUzi false)))
          (else
            (Utilities|IsValid (Variables|Default|GetPistolRef)
              (:Is%20Valid
                (Default|Throw (Variables|Default|GetPistolRef))
                (Transformation|DetachFromActor (Variables|Default|GetPistolRef) "KeepWorld" "KeepWorld" "KeepWorld")
                (Physics|AddImpulseatLocation (Variables|/Script/SuperHotProject.BaseWeapon|GetBoxComp (Variables|Default|GetPistolRef)) "500.000000,0.000000,0.000000" (- (Transformation|GetWorldLocation (Variables|/Script/SuperHotProject.BaseWeapon|GetBoxComp (Variables|Default|GetPistolRef))) "0.000000,10.000000,0.000000") "None")
                (Physics|AddImpulse (Variables|/Script/SuperHotProject.BaseWeapon|GetBoxComp (Variables|Default|GetPistolRef)) (* (Math|Vector|GetForwardVector (Transformation|GetWorldRotation (Variables|Default|GetVRCamera))) (Variables|Default|GetThrowVelocity)) "None" true)
                (Variables|Default|SetPistolRef 0)
                (Variables|Default|SetisWeaponEquipped false)
                (Variables|Default|SetisUsingShotgun false)
                (Variables|Default|SetisUsingUzi false))))))
      (Rendering|SetVisibility (Variables|Default|GetLeftHandMesh) true false)
      (Rendering|SetVisibility (Variables|Default|GetRightHandMesh) true false)
      (else
        (bind _outhit (Collision|BoxTraceByChannel _returnvalue _returnvalue2 "18.000000,18.000000,18.000000" (Variables|/Script/Engine.SceneComponent|GetRelativeRotation (Variables|Default|GetVRCamera)) "TraceTypeQuery1" true 0 "ForDuration"))
        (Utilities|FlowControl|Sequence
          (:then_0
            (bind _asbp_player_weapon_pistol (Utilities|Casting|CastToBP_PlayerWeapon_Pistol (.HitActor (Collision|BreakHitResult _outhit))))
            (Variables|Default|SetCurPistolBullet 5)
            (|AttachPistol _asbp_player_weapon_pistol _asbp_player_weapon_pistol)
            (Rendering|SetVisibility (Variables|Default|GetLeftHandMesh) false false)
            (Rendering|SetVisibility (Variables|Default|GetRightHandMesh) false false))
          (:then_1
            (bind _asbp_player_weapon_shotgun (Utilities|Casting|CastToBP_PlayerWeapon_Shotgun (.HitActor (Collision|BreakHitResult _outhit))))
            (Variables|Default|SetCurShotgunBullet 3)
            (|AttachShotgun _asbp_player_weapon_shotgun _asbp_player_weapon_shotgun)
            (Rendering|SetVisibility (Variables|Default|GetLeftHandMesh) false false)
            (Rendering|SetVisibility (Variables|Default|GetRightHandMesh) false false))
          (:then_2
            (bind _asbp_player_weapon_uzi (Utilities|Casting|CastToBP_PlayerWeapon_Uzi (.HitActor (Collision|BreakHitResult _outhit))))
            (Variables|Default|SetCurUziBullet 15)
            (|AttachUzi _asbp_player_weapon_uzi _asbp_player_weapon_uzi)
            (Rendering|SetVisibility (Variables|Default|GetLeftHandMesh) false false)
            (Rendering|SetVisibility (Variables|Default|GetRightHandMesh) false false)))))))

(event Input|EnhancedActionEvents|EnhancedInputActionIA_Hand_Point_Left
  (params (ActionValue :type Float%20%28double-precision%29) (ElapsedSeconds :type Float%20%28double-precision%29) (TriggeredSeconds :type Float%20%28double-precision%29) (InputAction :type Input%20Action%20Object%20Reference :default "/Game/VRTemplate/Input/Actions/Hands/IA_Hand_Point_Left.IA_Hand_Point_Left"))
  (bind _lefthandmesh (Variables|Default|GetLeftHandMesh))
  (:Started
    (bind _asabp_mannequins_xr (Utilities|Casting|CastToABP_MannequinsXR (Components|SkeletalMesh|GetAnimInstance _lefthandmesh) :!label _label))
    (Variables|/Game/Characters/MannequinsXR/Meshes/ABP_MannequinsXR.ABP_MannequinsXR_C|SetPoseAlphaPoint _asabp_mannequins_xr 0.0))
  (:Canceled
    (goto _label))
  (:Completed
    (bind _asabp_mannequins_xr_2 (Utilities|Casting|CastToABP_MannequinsXR (Components|SkeletalMesh|GetAnimInstance _lefthandmesh)))
    (Variables|/Game/Characters/MannequinsXR/Meshes/ABP_MannequinsXR.ABP_MannequinsXR_C|SetPoseAlphaPoint _asabp_mannequins_xr_2 1.0)))

(event Input|EnhancedActionEvents|EnhancedInputActionIA_Hand_ThumbUp_Left
  (params (ActionValue :type Float%20%28double-precision%29) (ElapsedSeconds :type Float%20%28double-precision%29) (TriggeredSeconds :type Float%20%28double-precision%29) (InputAction :type Input%20Action%20Object%20Reference :default "/Game/VRTemplate/Input/Actions/Hands/IA_Hand_ThumbUp_Left.IA_Hand_ThumbUp_Left"))
  (bind _lefthandmesh (Variables|Default|GetLeftHandMesh))
  (:Started
    (bind _asabp_mannequins_xr (Utilities|Casting|CastToABP_MannequinsXR (Components|SkeletalMesh|GetAnimInstance _lefthandmesh) :!label _label))
    (Variables|/Game/Characters/MannequinsXR/Meshes/ABP_MannequinsXR.ABP_MannequinsXR_C|SetPoseAlphaThumbUp _asabp_mannequins_xr 0.0))
  (:Canceled
    (goto _label))
  (:Completed
    (bind _asabp_mannequins_xr_2 (Utilities|Casting|CastToABP_MannequinsXR (Components|SkeletalMesh|GetAnimInstance _lefthandmesh)))
    (Variables|/Game/Characters/MannequinsXR/Meshes/ABP_MannequinsXR.ABP_MannequinsXR_C|SetPoseAlphaThumbUp _asabp_mannequins_xr_2 1.0)))

(event Input|EnhancedActionEvents|EnhancedInputActionIA_Hand_IndexCurl_Right
  (params (ActionValue :type Float%20%28double-precision%29) (ElapsedSeconds :type Float%20%28double-precision%29) (TriggeredSeconds :type Float%20%28double-precision%29) (InputAction :type Input%20Action%20Object%20Reference :default "/Game/VRTemplate/Input/Actions/Hands/IA_Hand_IndexCurl_Right.IA_Hand_IndexCurl_Right"))
  (bind _righthandmesh (Variables|Default|GetRightHandMesh))
  (bind _returnvalue (Components|SkeletalMesh|GetAnimInstance _righthandmesh))
  (:Triggered
    (bind _asabp_mannequins_xr (Utilities|Casting|CastToABP_MannequinsXR _returnvalue))
    (Variables|/Game/Characters/MannequinsXR/Meshes/ABP_MannequinsXR.ABP_MannequinsXR_C|SetPoseAlphaIndexCurl _asabp_mannequins_xr ActionValue))
  (:Canceled
    (bind _asabp_mannequins_xr_2 (Utilities|Casting|CastToABP_MannequinsXR _returnvalue :!label _label))
    (Variables|/Game/Characters/MannequinsXR/Meshes/ABP_MannequinsXR.ABP_MannequinsXR_C|SetPoseAlphaIndexCurl _asabp_mannequins_xr_2 0.0))
  (:Completed
    (goto _label)))

(event Input|EnhancedActionEvents|EnhancedInputActionIA_Hand_Grasp_Right
  (params (ActionValue :type Float%20%28double-precision%29) (ElapsedSeconds :type Float%20%28double-precision%29) (TriggeredSeconds :type Float%20%28double-precision%29) (InputAction :type Input%20Action%20Object%20Reference :default "/Game/VRTemplate/Input/Actions/Hands/IA_Hand_Grasp_Right.IA_Hand_Grasp_Right"))
  (bind _righthandmesh (Variables|Default|GetRightHandMesh))
  (bind _returnvalue (Components|SkeletalMesh|GetAnimInstance _righthandmesh))
  (:Triggered
    (bind _asabp_mannequins_xr (Utilities|Casting|CastToABP_MannequinsXR _returnvalue))
    (Variables|/Game/Characters/MannequinsXR/Meshes/ABP_MannequinsXR.ABP_MannequinsXR_C|SetPoseAlphaGrasp _asabp_mannequins_xr ActionValue))
  (:Canceled
    (bind _asabp_mannequins_xr_2 (Utilities|Casting|CastToABP_MannequinsXR _returnvalue :!label _label))
    (Variables|/Game/Characters/MannequinsXR/Meshes/ABP_MannequinsXR.ABP_MannequinsXR_C|SetPoseAlphaGrasp _asabp_mannequins_xr_2 0.0))
  (:Completed
    (goto _label)))

(event Input|EnhancedActionEvents|EnhancedInputActionIA_Hand_IndexCurl_Left
  (params (ActionValue :type Float%20%28double-precision%29) (ElapsedSeconds :type Float%20%28double-precision%29) (TriggeredSeconds :type Float%20%28double-precision%29) (InputAction :type Input%20Action%20Object%20Reference :default "/Game/VRTemplate/Input/Actions/Hands/IA_Hand_IndexCurl_Left.IA_Hand_IndexCurl_Left"))
  (bind _lefthandmesh (Variables|Default|GetLeftHandMesh))
  (bind _returnvalue (Components|SkeletalMesh|GetAnimInstance _lefthandmesh))
  (:Triggered
    (bind _asabp_mannequins_xr (Utilities|Casting|CastToABP_MannequinsXR _returnvalue))
    (Variables|/Game/Characters/MannequinsXR/Meshes/ABP_MannequinsXR.ABP_MannequinsXR_C|SetPoseAlphaIndexCurl _asabp_mannequins_xr ActionValue))
  (:Canceled
    (bind _asabp_mannequins_xr_2 (Utilities|Casting|CastToABP_MannequinsXR _returnvalue :!label _label))
    (Variables|/Game/Characters/MannequinsXR/Meshes/ABP_MannequinsXR.ABP_MannequinsXR_C|SetPoseAlphaIndexCurl _asabp_mannequins_xr_2 0.0))
  (:Completed
    (goto _label)))

(event Input|EnhancedActionEvents|EnhancedInputActionIA_Hand_ThumbUp_Right
  (params (ActionValue :type Float%20%28double-precision%29) (ElapsedSeconds :type Float%20%28double-precision%29) (TriggeredSeconds :type Float%20%28double-precision%29) (InputAction :type Input%20Action%20Object%20Reference :default "/Game/VRTemplate/Input/Actions/Hands/IA_Hand_ThumbUp_Right.IA_Hand_ThumbUp_Right"))
  (bind _righthandmesh (Variables|Default|GetRightHandMesh))
  (:Started
    (bind _asabp_mannequins_xr (Utilities|Casting|CastToABP_MannequinsXR (Components|SkeletalMesh|GetAnimInstance _righthandmesh) :!label _label))
    (Variables|/Game/Characters/MannequinsXR/Meshes/ABP_MannequinsXR.ABP_MannequinsXR_C|SetPoseAlphaThumbUp _asabp_mannequins_xr 0.0))
  (:Canceled
    (goto _label))
  (:Completed
    (bind _asabp_mannequins_xr_2 (Utilities|Casting|CastToABP_MannequinsXR (Components|SkeletalMesh|GetAnimInstance _righthandmesh)))
    (Variables|/Game/Characters/MannequinsXR/Meshes/ABP_MannequinsXR.ABP_MannequinsXR_C|SetPoseAlphaThumbUp _asabp_mannequins_xr_2 1.0)))

(event Input|EnhancedActionEvents|EnhancedInputActionIA_Hand_Point_Right
  (params (ActionValue :type Float%20%28double-precision%29) (ElapsedSeconds :type Float%20%28double-precision%29) (TriggeredSeconds :type Float%20%28double-precision%29) (InputAction :type Input%20Action%20Object%20Reference :default "/Game/VRTemplate/Input/Actions/Hands/IA_Hand_Point_Right.IA_Hand_Point_Right"))
  (bind _righthandmesh (Variables|Default|GetRightHandMesh))
  (:Started
    (bind _asabp_mannequins_xr (Utilities|Casting|CastToABP_MannequinsXR (Components|SkeletalMesh|GetAnimInstance _righthandmesh) :!label _label))
    (Variables|/Game/Characters/MannequinsXR/Meshes/ABP_MannequinsXR.ABP_MannequinsXR_C|SetPoseAlphaPoint _asabp_mannequins_xr 0.0))
  (:Canceled
    (goto _label))
  (:Completed
    (bind _asabp_mannequins_xr_2 (Utilities|Casting|CastToABP_MannequinsXR (Components|SkeletalMesh|GetAnimInstance _righthandmesh)))
    (Variables|/Game/Characters/MannequinsXR/Meshes/ABP_MannequinsXR.ABP_MannequinsXR_C|SetPoseAlphaPoint _asabp_mannequins_xr_2 1.0)))

(event EventDetachPistol)

(event EventResetFireCooldown
  (Utilities|FlowControl|Delay (Variables|Default|GetTimeBetweenShots))
  (Audio|PlaySound2D "/Game/KHJContent/Sounds/pistol_pickup.pistol_pickup" 1.0 1.0 0.0 0 0 false)
  (Utilities|FlowControl|Delay 0.1)
  (Variables|Default|SetbCanFire true))

(event EventBeginPlay
  (bind _asabp_mannequins_xr (Utilities|Casting|CastToABP_MannequinsXR (Components|SkeletalMesh|GetAnimInstance (Variables|Default|GetLeftHandMesh))))
  (Variables|/Game/Characters/MannequinsXR/Meshes/ABP_MannequinsXR.ABP_MannequinsXR_C|SetbMirror _asabp_mannequins_xr true)
  (bind _returnvalue (Game|SpawnActorfromClass "/Game/KHJContent/MyBlueprint/BP_PlayerWeapon_Pistol.BP_PlayerWeapon_Pistol_C" (Math|Transform|MakeTransform "0.000000,0.000000,-500.000000" "0, 0, 0" "1.000000,1.000000,1.000000") "Undefined" 0 0))
  (Variables|Default|SetPistolRef _returnvalue)
  (bind _returnvalue_2 (Game|SpawnActorfromClass "/Game/KHJContent/MyBlueprint/BP_PlayerWeapon_Shotgun.BP_PlayerWeapon_Shotgun_C" (Math|Transform|MakeTransform "0.000000,0.000000,-500.000000" "0, 0, 0" "1.000000,1.000000,1.000000") "Undefined" 0 0))
  (Variables|Default|SetShotgunRef _returnvalue_2)
  (bind _returnvalue_3 (Game|SpawnActorfromClass "/Game/KHJContent/MyBlueprint/BP_PlayerWeapon_Uzi.BP_PlayerWeapon_Uzi_C" (Math|Transform|MakeTransform "0.000000,0.000000,-500.000000" "0, 0, 0" "1.000000,1.000000,1.000000") "Undefined" 0 0))
  (Variables|Default|SetUziRef _returnvalue_3))

(event Collision|EventActorBeginOverlap
  (params (OtherActor :type Actor%20Object%20Reference)))

(event EventSpawnShotgunBullet
  (Default|SpawnBullet (Variables|Default|GetShotgunRef)))

(event EventSpawnPistolBullet
  (Default|SpawnBullet (Variables|Default|GetPistolRef)))

(event EventTick
  (params (DeltaSeconds :type Float%20%28single-precision%29)))

(event Input|ActionEvents|InputActionTestKey
  (params (Key :type Key%20Structure :default "None"))
  (:Pressed
    (Utilities|FlowControl|FlipFlop
      (:A
        (Variables|Default|SetbTestTime true))
      (:B
        (Variables|Default|SetbTestTime false)))))

(event Input|ActionEvents|InputActionAttach
  (params (Key :type Key%20Structure :default "None"))
  (bind (_returnvalue _returnvalue2) (|LineTraceLoc))
  (:Pressed
    (if (Variables|Default|GetisWeaponEquipped)
      (if (Variables|Default|GetisUsingShotgun)
        (Utilities|IsValid (Variables|Default|GetShotgunRef)
          (:Is%20Valid
            (Default|Throw (Variables|Default|GetShotgunRef))
            (Transformation|DetachFromActor (Variables|Default|GetShotgunRef) "KeepWorld" "KeepWorld" "KeepWorld")
            (Physics|AddImpulseatLocation (Variables|/Script/SuperHotProject.BaseWeapon|GetBoxComp (Variables|Default|GetShotgunRef)) "500.000000,0.000000,0.000000" (- (Transformation|GetWorldLocation (Variables|/Script/SuperHotProject.BaseWeapon|GetBoxComp (Variables|Default|GetShotgunRef))) "0.000000,10.000000,0.000000") "None")
            (Physics|AddImpulse (Variables|/Script/SuperHotProject.BaseWeapon|GetBoxComp (Variables|Default|GetShotgunRef)) (* (Math|Vector|GetForwardVector (Transformation|GetWorldRotation (Variables|Default|GetVRCamera))) (Variables|Default|GetThrowVelocity)) "None" true)
            (Variables|Default|SetShotgunRef 0)
            (Variables|Default|SetisWeaponEquipped false)
            (Variables|Default|SetisUsingShotgun false)
            (Variables|Default|SetisUsingUzi false)))
        (elif (Variables|Default|GetisUsingUzi)
          (Utilities|IsValid (Variables|Default|GetUziRef)
            (:Is%20Valid
              (Default|Throw (Variables|Default|GetUziRef))
              (Transformation|DetachFromActor (Variables|Default|GetUziRef) "KeepWorld" "KeepWorld" "KeepWorld")
              (Physics|AddImpulseatLocation (Variables|/Script/SuperHotProject.BaseWeapon|GetBoxComp (Variables|Default|GetUziRef)) "500.000000,0.000000,0.000000" (- (Transformation|GetWorldLocation (Variables|/Script/SuperHotProject.BaseWeapon|GetBoxComp (Variables|Default|GetUziRef))) "0.000000,10.000000,0.000000") "None")
              (Physics|AddImpulse (Variables|/Script/SuperHotProject.BaseWeapon|GetBoxComp (Variables|Default|GetUziRef)) (* (Math|Vector|GetForwardVector (Transformation|GetWorldRotation (Variables|Default|GetVRCamera))) (Variables|Default|GetThrowVelocity)) "None" true)
              (Variables|Default|SetUziRef 0)
              (Variables|Default|SetisWeaponEquipped false)
              (Variables|Default|SetisUsingShotgun false)
              (Variables|Default|SetisUsingUzi false)))
          (else
            (Utilities|IsValid (Variables|Default|GetPistolRef)
              (:Is%20Valid
                (Default|Throw (Variables|Default|GetPistolRef))
                (Transformation|DetachFromActor (Variables|Default|GetPistolRef) "KeepWorld" "KeepWorld" "KeepWorld")
                (Physics|AddImpulseatLocation (Variables|/Script/SuperHotProject.BaseWeapon|GetBoxComp (Variables|Default|GetPistolRef)) "500.000000,0.000000,0.000000" (- (Transformation|GetWorldLocation (Variables|/Script/SuperHotProject.BaseWeapon|GetBoxComp (Variables|Default|GetPistolRef))) "0.000000,10.000000,0.000000") "None")
                (Physics|AddImpulse (Variables|/Script/SuperHotProject.BaseWeapon|GetBoxComp (Variables|Default|GetPistolRef)) (* (Math|Vector|GetForwardVector (Transformation|GetWorldRotation (Variables|Default|GetVRCamera))) (Variables|Default|GetThrowVelocity)) "None" true)
                (Variables|Default|SetPistolRef 0)
                (Variables|Default|SetisWeaponEquipped false)
                (Variables|Default|SetisUsingShotgun false)
                (Variables|Default|SetisUsingUzi false))))))
      (Rendering|SetVisibility (Variables|Default|GetLeftHandMesh) true false)
      (Rendering|SetVisibility (Variables|Default|GetRightHandMesh) true false)
      (else
        (bind _outhit (Collision|BoxTraceByChannel _returnvalue _returnvalue2 "18.000000,18.000000,18.000000" (Variables|/Script/Engine.SceneComponent|GetRelativeRotation (Variables|Default|GetVRCamera)) "TraceTypeQuery1" true 0 "ForDuration"))
        (Utilities|FlowControl|Sequence
          (:then_0
            (bind _asbp_player_weapon_pistol (Utilities|Casting|CastToBP_PlayerWeapon_Pistol (.HitActor (Collision|BreakHitResult _outhit))))
            (Variables|Default|SetCurPistolBullet 5)
            (|AttachPistol _asbp_player_weapon_pistol _asbp_player_weapon_pistol)
            (Rendering|SetVisibility (Variables|Default|GetLeftHandMesh) false false)
            (Rendering|SetVisibility (Variables|Default|GetRightHandMesh) false false))
          (:then_1
            (bind _asbp_player_weapon_shotgun (Utilities|Casting|CastToBP_PlayerWeapon_Shotgun (.HitActor (Collision|BreakHitResult _outhit))))
            (Variables|Default|SetCurShotgunBullet 3)
            (|AttachShotgun _asbp_player_weapon_shotgun _asbp_player_weapon_shotgun)
            (Rendering|SetVisibility (Variables|Default|GetLeftHandMesh) false false)
            (Rendering|SetVisibility (Variables|Default|GetRightHandMesh) false false))
          (:then_2
            (bind _asbp_player_weapon_uzi (Utilities|Casting|CastToBP_PlayerWeapon_Uzi (.HitActor (Collision|BreakHitResult _outhit))))
            (Variables|Default|SetCurUziBullet 15)
            (|AttachUzi _asbp_player_weapon_uzi _asbp_player_weapon_uzi)
            (Rendering|SetVisibility (Variables|Default|GetLeftHandMesh) false false)
            (Rendering|SetVisibility (Variables|Default|GetRightHandMesh) false false)))))))

(fn ConstructionScript)

(fn IsMoving
  (return (or (!= (Variables|Default|GetXMovement) 0.0) (!= (Variables|Default|GetYMovement) 0.0))))

(fn PickUpPistol
  (params (HeldWeapon :type BP%20Player%20Weapon%20Pistol%20Object%20Reference))
  (bind _output_get (Variables|Default|SetPistolRef HeldWeapon))
  (Transformation|AttachComponentToComponent (Variables|/Script/Engine.Actor|GetRootComponent _output_get) (Variables|Default|GetRightHandMesh) "Weapon_R" "SnapToTarget" "SnapToTarget" "SnapToTarget" true)
  (Default|Collected (Variables|Default|GetPistolRef))
  (Variables|Default|SetisWeaponEquipped true)
  (Variables|Default|SetisUsingShotgun false)
  (Variables|Default|SetisUsingUzi false))

(fn PickupGun
  (params (HeldWeapon :type %20Object%20Reference)))

(fn PickUpShotgun
  (params (ShotgunRef :type BP%20Player%20Weapon%20Shotgun%20Object%20Reference))
  (bind _output_get (Variables|Default|SetShotgunRef ShotgunRef))
  (Transformation|AttachComponentToComponent (Variables|/Script/Engine.Actor|GetRootComponent _output_get) (Variables|Default|GetRightHandMesh) "Weapon_R1" "SnapToTarget" "SnapToTarget" "SnapToTarget" true)
  (Default|Collected (Variables|Default|GetShotgunRef))
  (Variables|Default|SetisWeaponEquipped true)
  (Variables|Default|SetisUsingShotgun true)
  (Variables|Default|SetisUsingUzi false))

(fn PickUpUzi
  (params (UziRef :type BP%20Player%20Weapon%20Uzi%20Object%20Reference))
  (bind _output_get (Variables|Default|SetUziRef UziRef))
  (Transformation|AttachComponentToComponent (Variables|/Script/Engine.Actor|GetRootComponent _output_get) (Variables|Default|GetRightHandMesh) "Weapon_R2" "SnapToTarget" "SnapToTarget" "SnapToTarget" true)
  (Default|Collected (Variables|Default|GetUziRef))
  (Variables|Default|SetisWeaponEquipped true)
  (Variables|Default|SetisUsingShotgun false)
  (Variables|Default|SetisUsingUzi true))