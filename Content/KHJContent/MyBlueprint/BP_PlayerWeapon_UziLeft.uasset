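; Left-hand Uzi weapon for the player that can be collected, thrown and fired automatically.
; Box overlap with the player's attach box swaps in a highlight material, while Collected and Throw toggle physics and collision.
; Looping timers drive fire functions for right and left variants, each playing a sound, spawning a projectile at its socket and decrementing the player's matching ammo counter until empty clears the timer.
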(event OnComponentBeginOverlap(BoxComp)
  (params (OverlappedComponent :type Primitive%20Component%20Object%20Reference) (OtherActor :type Actor%20Object%20Reference) (OtherComp :type Primitive%20Component%20Object%20Reference) (OtherBodyIndex :type Integer) (bFromSweep :type Boolean) (SweepResult :type Hit%20Result%20Structure%20%28by%20ref%29))
  (bind _asplayer_character (Utilities|Casting|CastToPlayerCharacter (Game|GetPlayerCharacter 0)))
  (if (Class|PrimitiveComponent|IsOverlappingComponent (Variables|Default|GetBoxComp) (Variables|/Script/SuperHotProject.PlayerCharacter|GetattachBoxComp _asplayer_character))
    (Rendering|Material|SetMaterial (Variables|Default|GetuziComp) 0 "/Game/Assets/Materials/M_OvelappedSpecBlack_Inst1.M_OvelappedSpecBlack_Inst1")))

(event OnComponentEndOverlap(BoxComp)
  (params (OverlappedComponent :type Primitive%20Component%20Object%20Reference) (OtherActor :type Actor%20Object%20Reference) (OtherComp :type Primitive%20Component%20Object%20Reference) (OtherBodyIndex :type Integer))
  (bind _asplayer_character (Utilities|Casting|CastToPlayerCharacter (Game|GetPlayerCharacter 0)))
  (if (not (Class|PrimitiveComponent|IsOverlappingComponent (Variables|Default|GetBoxComp) (Variables|/Script/SuperHotProject.PlayerCharacter|GetattachBoxComp _asplayer_character)))
    (Rendering|Material|SetMaterial (Variables|Default|GetuziComp) 0 "/Game/Assets/Materials/M_SpecBlack_Inst.M_SpecBlack_Inst")))

(event EventBeginPlay
  (bind _asplayer_character (Utilities|Casting|CastToPlayerCharacter (Game|GetPlayerCharacter 0)))
  (Variables|Default|SetAs%20Player%20Character _asplayer_character))

(fn ConstructionScript)

(fn Collected
  (bind _boxcomp (Variables|Default|GetBoxComp))
  (Class|PrimitiveComponent|SetAllPhysicsLinearVelocity (Variables|Default|GetBoxComp) "0, 0, 0" false)
  (Physics|SetSimulatePhysics _boxcomp false)
  (Collision|SetCollisionEnabled _boxcomp "NoCollision"))

(fn Throw
  (bind _boxcomp (Variables|Default|GetBoxComp))
  (Physics|SetSimulatePhysics _boxcomp true)
  (Collision|SetCollisionEnabled _boxcomp "QueryAndPhysics")
  (Collision|SetCollisionResponsetoAllChannels (Variables|Default|GetBoxComp) "ECR_Block"))

(fn SpawnBullet
  (bind _returnvalue (Utilities|Time|SetTimerbyEvent (EventDispatchers|CreateEvent :!event BPPlayerWeaponUziAutoGenFunc) 0.1 true))
  (Variables|Default|SetFTimerHandle _returnvalue))

(fn BPPlayerWeaponUziAutoGenFunc
  (bind _as_player_character (Variables|Default|GetAs%20Player%20Character))
  (Audio|PlaySound2D "/Game/KHJContent/Sounds/pistol_fire.pistol_fire" 1.0 1.5 0.0 0 0 false)
  (Game|SpawnActorfromClass "/Game/KHJContent/MyBlueprint/BP_Projectile.BP_Projectile_C" (Transformation|GetSocketTransform (Variables|Default|GetuziComp) "FireSocket" "RTS_World") "Undefined" 0 0)
  (Variables|/Script/SuperHotProject.PlayerCharacter|SetCurUziBullet _as_player_character (- (Variables|/Script/SuperHotProject.PlayerCharacter|GetCurUziBullet _as_player_character) 1))
  (if (<= (Variables|/Script/SuperHotProject.PlayerCharacter|GetCurUziBullet (Variables|Default|GetAs%20Player%20Character)) 0)
    (Utilities|Time|ClearandInvalidateTimerbyHandle (Variables|Default|GetFTimerHandle))))

(fn SpawnBulletLeft
  (bind _returnvalue (Utilities|Time|SetTimerbyEvent (EventDispatchers|CreateEvent :!event BPPlayerWeaponUziAutoGenFuncLeft) 0.1 true))
  (Variables|Default|SetFTimerHandle _returnvalue))

(fn BPPlayerWeaponUziAutoGenFuncLeft
  (bind _as_player_character (Variables|Default|GetAs%20Player%20Character))
  (Audio|PlaySound2D "/Game/KHJContent/Sounds/pistol_fire.pistol_fire" 1.0 1.5 0.0 0 0 false)
  (Game|SpawnActorfromClass "/Game/KHJContent/MyBlueprint/BP_Projectile.BP_Projectile_C" (Transformation|GetSocketTransform (Variables|Default|GetuziComp) "FireSocketLeft" "RTS_World") "Undefined" 0 0)
  (Variables|/Script/SuperHotProject.PlayerCharacter|SetCurUziBulletLeft _as_player_character (- (Variables|/Script/SuperHotProject.PlayerCharacter|GetCurUziBulletLeft _as_player_character) 1))
  (if (<= (Variables|/Script/SuperHotProject.PlayerCharacter|GetCurUziBulletLeft (Variables|Default|GetAs%20Player%20Character)) 0)
    (Utilities|Time|ClearandInvalidateTimerbyHandle (Variables|Default|GetFTimerHandle))))