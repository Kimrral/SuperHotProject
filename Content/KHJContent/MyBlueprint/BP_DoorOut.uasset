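; BP_DoorOut is an exit door that highlights when the player is near and quits the game when hit by a BP_PunchBoxComp actor.
; Its Box overlap events check the PlayerCharacter's AttachBoxComp to swap the mesh between a highlighted material and plain black.
; The begin-overlap event also casts the overlapping actor to BP_PunchBoxComp and calls QuitGame on success, but only after the player cast succeeds or fails independently via a Sequence.
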(event OnComponentBeginOverlap(Box)
  (params (OverlappedComponent :type Primitive%20Component%20Object%20Reference) (OtherActor :type Actor%20Object%20Reference) (OtherComp :type Primitive%20Component%20Object%20Reference) (OtherBodyIndex :type Integer) (bFromSweep :type Boolean) (SweepResult :type Hit%20Result%20Structure%20%28by%20ref%29))
  (Utilities|FlowControl|Sequence
    (:then_0
      (bind _asplayer_character (Utilities|Casting|CastToPlayerCharacter (Game|GetPlayerCharacter 0)))
      (if (Class|PrimitiveComponent|IsOverlappingComponent (Variables|Default|GetBox) (Variables|/Script/SuperHotProject.PlayerCharacter|GetattachBoxComp _asplayer_character))
        (Rendering|Material|SetMaterial (Variables|Default|GetStaticMesh) 0 "/Game/Assets/Materials/M_OvelappedSpecBlack_Inst1.M_OvelappedSpecBlack_Inst1")))
    (:then_1
      (Utilities|Casting|CastToBP_PunchBoxComp OtherActor)
      (Game|QuitGame 0 "Quit" false))))

(event OnComponentEndOverlap(Box)
  (params (OverlappedComponent :type Primitive%20Component%20Object%20Reference) (OtherActor :type Actor%20Object%20Reference) (OtherComp :type Primitive%20Component%20Object%20Reference) (OtherBodyIndex :type Integer))
  (bind _asplayer_character (Utilities|Casting|CastToPlayerCharacter (Game|GetPlayerCharacter 0)))
  (if (not (Class|PrimitiveComponent|IsOverlappingComponent (Variables|Default|GetBox) (Variables|/Script/SuperHotProject.PlayerCharacter|GetattachBoxComp _asplayer_character)))
    (Rendering|Material|SetMaterial (Variables|Default|GetStaticMesh) 0 "/Game/EF_Barbra/Materials/M_Black.M_Black")))

(event EventBeginPlay)

(event Collision|EventActorBeginOverlap
  (params (OtherActor :type Actor%20Object%20Reference)))

(event EventTick
  (params (DeltaSeconds :type Float%20%28single-precision%29)))

(fn ConstructionScript)