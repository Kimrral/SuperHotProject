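; BP_PlayerWeapon_Uzi is the player's Uzi weapon Blueprint, handling the physics state changes for being collected and thrown.
; Collected zeroes BoxComp's linear velocity, then turns off its physics simulation and collision.
; Throw re-enables simulation and query-and-physics collision, blocking all channels, without applying any impulse itself.
; The event graph and construction script contain no active logic.
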(event EventBeginPlay)

(event Collision|EventActorBeginOverlap
  (params (OtherActor :type Actor%20Object%20Reference)))

(event EventTick
  (params (DeltaSeconds :type Float%20%28single-precision%29)))

(fn ConstructionScript)

(fn Collected
  (bind _boxcomp (Variables|Default|GetBoxComp))
  (Class|PrimitiveComponent|SetAllPhysicsLinearVelocity (Variables|Default|GetBoxComp) "0, 0, 0" false)
  (Physics|SetSimulatePhysics _boxcomp false)
  (Collision|SetCollisionEnabled _boxcomp "NoCollision"))

(fn Throw
  (bind _boxcomp (Variables|Default|GetBoxComp))
  (Physics|SetSimulatePhysics _boxcomp true)
  (Collision|SetCollisionEnabled _boxcomp "QueryAndPhysics")
  (Collision|SetCollisionResponsetoAllChannels (Variables|Default|GetBoxComp) "ECR_Block"))