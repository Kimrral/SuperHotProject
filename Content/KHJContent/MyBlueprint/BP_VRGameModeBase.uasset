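; VR game mode that detects when all enemies are defeated and triggers the level-clear sequence.
; Tick checks whether spawning has started and the TotalEnemy count has reached zero.
; On the first such frame it shows the WB_Super widget, spawns a BP_GrabGC actor 400 units ahead of the player, then sets Clear so the sequence runs only once.
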(event EventBeginPlay)

(event EventTick
  (params (DeltaSeconds :type Float%20%28single-precision%29))
  (bind _returnvalue (Game|GetPlayerCharacter 0))
  (if (Variables|Default|GetbSpawn)
    (if (<= (Variables|Default|GettotalEnemy) 0)
      (if (not (Variables|Default|GetbClear))
        (bind _returnvalue_2 (UserInterface|CreateWidget "/Game/KHJContent/MyUI/WB_Super.WB_Super_C"))
        (UserInterface|Viewport|AddtoViewport _returnvalue_2 0)
        (Game|SpawnActorfromClass "/Game/MyeongSeok/Destruction/BP_GrabGC.BP_GrabGC_C" (Math|Conversions|ToTransform(Vector) (+ (Transformation|GetActorLocation _returnvalue) (* (Transformation|GetActorForwardVector _returnvalue) 4e+02))) "Undefined" 0 0)
        (Variables|Default|SetbClear true)))))

(fn ConstructionScript)