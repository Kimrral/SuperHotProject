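; BP_Enemy1 is a modular enemy whose body parts break off when hit by BP_Projectile.
; The construction script makes limb and body meshes follow Mesh, the head, as leader pose.
; Six overlap boxes each spawn a geometry actor and hide their part once; the right leg reuses BP_LeftLegGeometry.
; A body hit also clears the leader pose after a short delay and enables physics on all parts.
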(event OnComponentBeginOverlap(Box)
  (params (OverlappedComponent :type Primitive%20Component%20Object%20Reference) (OtherActor :type Actor%20Object%20Reference) (OtherComp :type Primitive%20Component%20Object%20Reference) (OtherBodyIndex :type Integer) (bFromSweep :type Boolean) (SweepResult :type Hit%20Result%20Structure%20%28by%20ref%29))
  (Utilities|Casting|CastToBP_Projectile OtherActor)
  (if (not (Variables|Default|GetisDestroyRightArm))
    (Game|SpawnActorfromClass "/Game/MyeongSeok/Destruction/BP_RightArmGeometry.BP_RightArmGeometry_C" (Math|Conversions|ToTransform(Vector) (Transformation|GetSocketLocation (Variables|Default|GetRightArm) "None")) "Undefined" 0 0)
    (Rendering|SetVisibility (Variables|Default|GetRightArm) false false)
    (Variables|Default|SetisDestroyRightArm true)))

(event OnComponentBeginOverlap(Box1)
  (params (OverlappedComponent :type Primitive%20Component%20Object%20Reference) (OtherActor :type Actor%20Object%20Reference) (OtherComp :type Primitive%20Component%20Object%20Reference) (OtherBodyIndex :type Integer) (bFromSweep :type Boolean) (SweepResult :type Hit%20Result%20Structure%20%28by%20ref%29))
  (Utilities|Casting|CastToBP_Projectile OtherActor)
  (if (not (Variables|Default|GetisDestroyLeftArm))
    (Game|SpawnActorfromClass "/Game/MyeongSeok/Destruction/BP_LeftArmGeometry.BP_LeftArmGeometry_C" (Math|Conversions|ToTransform(Vector) (Transformation|GetSocketLocation (Variables|Default|GetLeftArm) "root")) "Undefined" 0 0)
    (Rendering|SetVisibility (Variables|Default|GetLeftArm) false false)
    (Variables|Default|SetisDestroyLeftArm true)))

(event OnComponentBeginOverlap(Box2)
  (params (OverlappedComponent :type Primitive%20Component%20Object%20Reference) (OtherActor :type Actor%20Object%20Reference) (OtherComp :type Primitive%20Component%20Object%20Reference) (OtherBodyIndex :type Integer) (bFromSweep :type Boolean) (SweepResult :type Hit%20Result%20Structure%20%28by%20ref%29))
  (Utilities|Casting|CastToBP_Projectile OtherActor)
  (if (not (Variables|Default|GetisDestroyBody))
    (Game|SpawnActorfromClass "/Game/MyeongSeok/Destruction/BP_BodyGeometry.BP_BodyGeometry_C" (Math|Conversions|ToTransform(Vector) (Transformation|GetSocketLocation (Variables|Default|GetBody) "None")) "Undefined" 0 0)
    (Rendering|SetVisibility (Variables|Default|GetBody) false false)
    (Variables|Default|SetisDestroyBody true)
    (Utilities|FlowControl|Delay 0.3)
    (Components|SkinnedMesh|SetLeaderPoseComponent (Variables|Default|GetLeftLeg) 0 false false)
    (Physics|SetSimulatePhysics (Variables|Character|GetMesh) true)))

(event OnComponentBeginOverlap(Box3)
  (params (OverlappedComponent :type Primitive%20Component%20Object%20Reference) (OtherActor :type Actor%20Object%20Reference) (OtherComp :type Primitive%20Component%20Object%20Reference) (OtherBodyIndex :type Integer) (bFromSweep :type Boolean) (SweepResult :type Hit%20Result%20Structure%20%28by%20ref%29))
  (Utilities|Casting|CastToBP_Projectile OtherActor)
  (if (not (Variables|Default|GetisDestroyHead))
    (Game|SpawnActorfromClass "/Game/MyeongSeok/Destruction/BP_HeadGeometry.BP_HeadGeometry_C" (Math|Conversions|ToTransform(Vector) (Transformation|GetSocketLocation (Variables|Character|GetMesh) "root")) "Undefined" 0 0)
    (Rendering|SetVisibility (Variables|Character|GetMesh) false false)
    (Variables|Default|SetisDestroyHead true)))

(event OnComponentBeginOverlap(Box4)
  (params (OverlappedComponent :type Primitive%20Component%20Object%20Reference) (OtherActor :type Actor%20Object%20Reference) (OtherComp :type Primitive%20Component%20Object%20Reference) (OtherBodyIndex :type Integer) (bFromSweep :type Boolean) (SweepResult :type Hit%20Result%20Structure%20%28by%20ref%29))
  (Utilities|Casting|CastToBP_Projectile OtherActor)
  (if (not (Variables|Default|GetisDestroyLeftLeg))
    (Game|SpawnActorfromClass "/Game/MyeongSeok/Destruction/BP_LeftLegGeometry.BP_LeftLegGeometry_C" (Math|Conversions|ToTransform(Vector) (Transformation|GetSocketLocation (Variables|Default|GetLeftLeg) "root")) "Undefined" 0 0)
    (Rendering|SetVisibility (Variables|Default|GetLeftLeg) false false)
    (Variables|Default|SetisDestroyLeftLeg true)))

(event OnComponentBeginOverlap(Box5)
  (params (OverlappedComponent :type Primitive%20Component%20Object%20Reference) (OtherActor :type Actor%20Object%20Reference) (OtherComp :type Primitive%20Component%20Object%20Reference) (OtherBodyIndex :type Integer) (bFromSweep :type Boolean) (SweepResult :type Hit%20Result%20Structure%20%28by%20ref%29))
  (Utilities|Casting|CastToBP_Projectile OtherActor)
  (if (not (Variables|Default|GetisDestroyRightLeg))
    (Game|SpawnActorfromClass "/Game/MyeongSeok/Destruction/BP_LeftLegGeometry.BP_LeftLegGeometry_C" (Math|Conversions|ToTransform(Vector) (Transformation|GetSocketLocation (Variables|Default|GetRightLeg) "root")) "Undefined" 0 0)
    (Rendering|SetVisibility (Variables|Default|GetRightLeg) false false)
    (Variables|Default|SetisDestroyRightLeg true)))

(event Collision|EventActorBeginOverlap
  (params (OtherActor :type Actor%20Object%20Reference)))

(event EventTick
  (params (DeltaSeconds :type Float%20%28single-precision%29)))

(event EventBeginPlay)

(fn ConstructionScript
  (Components|SkinnedMesh|SetLeaderPoseComponent (Variables|Default|GetBody) (Variables|Character|GetMesh) false false))